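; Interactable world object that the player can highlight and inspect by rotating its mesh.
; Sphere overlaps with the player notify its AC_InteractionComponent, passing true on both begin and end, while hover events toggle a custom-depth outline.
; StartInspection moves input from the inspector to the object, where mouse drag with either button rolls and pitches the mesh.
; InteractKey returns input and calls Inspect on BP_FirstPersonCharacter.
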(event OnComponentBeginOverlap(Sphere)
  (params (OverlappedComponent :type Primitive%20Component%20Object%20Reference) (OtherActor :type Actor%20Object%20Reference) (OtherComp :type Primitive%20Component%20Object%20Reference) (OtherBodyIndex :type Integer) (bFromSweep :type Boolean) (SweepResult :type Hit%20Result%20Structure%20%28by%20ref%29))
  (bind _returnvalue (Actor|GetComponentbyClass OtherActor "/Game/GameObjects/AC_InteractionComponent.AC_InteractionComponent_C"))
  ;[0.15 0.15 0.15 0.5] Begin overlaps
  (if (== OtherActor (Game|GetPlayerCharacter 0))
    (if (Utilities|IsValid _returnvalue)
      (Default|OnInteractableOberlap _returnvalue true))))

(event OnComponentEndOverlap(Sphere)
  (params (OverlappedComponent :type Primitive%20Component%20Object%20Reference) (OtherActor :type Actor%20Object%20Reference) (OtherComp :type Primitive%20Component%20Object%20Reference) (OtherBodyIndex :type Integer))
  (bind _returnvalue (Actor|GetComponentbyClass OtherActor "/Game/GameObjects/AC_InteractionComponent.AC_InteractionComponent_C"))
  ;[0.15 0.15 0.15 0.5] End Overlaps
  (if (== OtherActor (Game|GetPlayerCharacter 0))
    (if (Utilities|IsValid _returnvalue)
      (Default|OnInteractableOberlap _returnvalue true))))

(event Custom|HightlightOverline
  (params (Show :type Boolean))
  (Rendering|SetRenderCustomDepth (Variables|Default|GetInteractableMesh) Show))

(event Custom|StartInspection
  (params (Inspector :type Pawn%20Object%20Reference))
  (bind _returnvalue (Game|GetPlayerController 0))
  (Input|DisableInput Inspector _returnvalue)
  (Input|EnableInput _returnvalue))

(event EventBeginPlay)

(event Collision|EventActorBeginOverlap
  (params (OtherActor :type Actor%20Object%20Reference)))

(event EventTick
  (params (DeltaSeconds :type Float%20%28single-precision%29)))

(event EventOnHovered
  (CallFunction|HightlightOverline true))

(event EventOnUnhovered
  (CallFunction|HightlightOverline false))

(event Input|ActionEvents|InputActionInteractKey
  (params (Key :type Key%20Structure :default "None"))
  (bind _returnvalue (Game|GetPlayerController 0))
  (:Pressed
    (Input|DisableInput _returnvalue)
    (Input|EnableInput (stale Custom|StartInspection Inspector) _returnvalue)
    (bind _asbp_first_person_character (Utilities|Casting|CastToBP_FirstPersonCharacter (stale Custom|StartInspection Inspector)))
    (Default|Inspect _asbp_first_person_character)))

(event Input|MouseEvents|MouseX
  (params (AxisValue :type Float%20%28single-precision%29))
  (bind _returnvalue (Game|GetPlayerController 0))
  (if (or (Game|Player|IsInputKeyDown _returnvalue "LeftMouseButton") (Game|Player|IsInputKeyDown _returnvalue "RightMouseButton"))
    (Transformation|SetRelativeRotation (Variables|Default|GetInteractableMesh) (Math|Rotator|CombineRotators (Variables|/Script/Engine.SceneComponent|GetRelativeRotation (Variables|Default|GetInteractableMesh)) (Math|Rotator|MakeRotator (* AxisValue -1.0) 0.0 0.0)) false false)))

(event Input|MouseEvents|MouseY
  (params (AxisValue :type Float%20%28single-precision%29))
  (bind _returnvalue (Game|GetPlayerController 0))
  (if (or (Game|Player|IsInputKeyDown _returnvalue "LeftMouseButton") (Game|Player|IsInputKeyDown _returnvalue "RightMouseButton"))
    (Transformation|SetRelativeRotation (Variables|Default|GetInteractableMesh) (Math|Rotator|CombineRotators (Variables|/Script/Engine.SceneComponent|GetRelativeRotation (Variables|Default|GetInteractableMesh)) (Math|Rotator|MakeRotator 0.0 (* AxisValue -1.0) 0.0)) false false)))

(fn ConstructionScript)