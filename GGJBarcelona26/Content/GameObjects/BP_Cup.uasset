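; BP_Cup is an interactable cup that receives the object the player is holding.
; Sphere overlaps notify the player's AC_InteractionComponent, passing true on both begin and end, while hover events toggle a custom-depth outline.
; On InteractKey, a short camera trace checks for a "Cup"-tagged actor.
; If the player is holding something, one sequence spawns and attaches copies at all four N, S, E and W points, destroying the held original.
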(event OnComponentBeginOverlap(Sphere)
  (params (OverlappedComponent :type Primitive%20Component%20Object%20Reference) (OtherActor :type Actor%20Object%20Reference) (OtherComp :type Primitive%20Component%20Object%20Reference) (OtherBodyIndex :type Integer) (bFromSweep :type Boolean) (SweepResult :type Hit%20Result%20Structure%20%28by%20ref%29))
  (bind _returnvalue (Actor|GetComponentbyClass OtherActor "/Game/GameObjects/AC_InteractionComponent.AC_InteractionComponent_C"))
  ;[0.15 0.15 0.15 0.5] Begin overlaps
  (if (== OtherActor (Game|GetPlayerCharacter 0))
    (if (Utilities|IsValid _returnvalue)
      (Default|OnInteractableOberlap _returnvalue true))))

(event OnComponentEndOverlap(Sphere)
  (params (OverlappedComponent :type Primitive%20Component%20Object%20Reference) (OtherActor :type Actor%20Object%20Reference) (OtherComp :type Primitive%20Component%20Object%20Reference) (OtherBodyIndex :type Integer))
  (bind _returnvalue (Actor|GetComponentbyClass OtherActor "/Game/GameObjects/AC_InteractionComponent.AC_InteractionComponent_C"))
  ;[0.15 0.15 0.15 0.5] End Overlaps
  (if (== OtherActor (Game|GetPlayerCharacter 0))
    (if (Utilities|IsValid _returnvalue)
      (Default|OnInteractableOberlap _returnvalue true))))

(event Custom|HightlightOverline
  (params (Show :type Boolean))
  (Rendering|SetRenderCustomDepth (Variables|Default|GetInteractableMesh) Show))

(event EventBeginPlay)

(event Collision|EventActorBeginOverlap
  (params (OtherActor :type Actor%20Object%20Reference)))

(event EventTick
  (params (DeltaSeconds :type Float%20%28single-precision%29)))

(event EventOnHovered
  (CallFunction|HightlightOverline true))

(event EventOnUnhovered
  (CallFunction|HightlightOverline false))

(event Input|ActionEvents|InputActionInteractKey
  (params (Key :type Key%20Structure :default "None"))
  (:Pressed
    (bind _outhit (Collision|LineTraceByChannel (Transformation|GetWorldLocation (Variables|/Game/FirstPerson/Blueprints/BP_FirstPersonCharacter.BP_FirstPersonCharacter_C|GetFirstPersonCamera (stale _asbp_first_person_character))) (+ (Transformation|GetWorldLocation (Variables|/Game/FirstPerson/Blueprints/BP_FirstPersonCharacter.BP_FirstPersonCharacter_C|GetFirstPersonCamera (stale _asbp_first_person_character))) (* (Math|Vector|GetForwardVector (Transformation|GetWorldRotation (Variables|/Game/FirstPerson/Blueprints/BP_FirstPersonCharacter.BP_FirstPersonCharacter_C|GetFirstPersonCamera (stale _asbp_first_person_character)))) 1.5e+02)) "TraceTypeQuery1" false 0 "None" true "(R=1.000000,G=0.000000,B=0.000000,A=1.000000)" "(R=0.000000,G=1.000000,B=0.000000,A=1.000000)" 1.0))
    (bind _asbp_first_person_character (Utilities|Casting|CastToBP_FirstPersonCharacter (Game|GetPlayerCharacter 0)))
    (if (Actor|ActorHasTag (.HitActor (Collision|BreakHitResult _outhit)) "Cup")
      (if (Variables|/Game/FirstPerson/Blueprints/BP_FirstPersonCharacter.BP_FirstPersonCharacter_C|GetHolding _asbp_first_person_character)
        (Variables|Default|SetHand%20Object (Variables|/Game/FirstPerson/Blueprints/BP_FirstPersonCharacter.BP_FirstPersonCharacter_C|GetHandObject _asbp_first_person_character))
        (Utilities|FlowControl|Sequence
          (:then_0
            (bind _returnvalue (Game|SpawnActorfromClass (Utilities|GetClass (Variables|Default|GetHand%20Object)) (Transformation|GetWorldTransform (Variables|Default|GetN)) "Undefined" "MultiplyWithRoot" 0 0))
            (Actor|DestroyActor (Variables|Default|GetHand%20Object))
            (Transformation|AttachComponentToComponent _returnvalue (Variables|Default|GetN) "None" "SnapToTarget" "SnapToTarget" "KeepWorld" true))
          (:then_1
            (bind _returnvalue_2 (Game|SpawnActorfromClass (Utilities|GetClass (Variables|Default|GetHand%20Object)) (Transformation|GetWorldTransform (Variables|Default|GetS)) "Undefined" "MultiplyWithRoot" 0 0))
            (Actor|DestroyActor (Variables|Default|GetHand%20Object))
            (Transformation|AttachComponentToComponent _returnvalue_2 (Variables|Default|GetS) "None" "SnapToTarget" "SnapToTarget" "KeepWorld" true))
          (:then_2
            (bind _returnvalue_3 (Game|SpawnActorfromClass (Utilities|GetClass (Variables|Default|GetHand%20Object)) (Transformation|GetWorldTransform (Variables|Default|GetE)) "Undefined" "MultiplyWithRoot" 0 0))
            (Actor|DestroyActor (Variables|Default|GetHand%20Object))
            (Transformation|AttachComponentToComponent _returnvalue_3 (Variables|Default|GetE) "None" "SnapToTarget" "SnapToTarget" "KeepWorld" true))
          (:then_3
            (bind _returnvalue_4 (Game|SpawnActorfromClass (Utilities|GetClass (Variables|Default|GetHand%20Object)) (Transformation|GetWorldTransform (Variables|Default|GetW)) "Undefined" "MultiplyWithRoot" 0 0))
            (Actor|DestroyActor (Variables|Default|GetHand%20Object))
            (Transformation|AttachComponentToComponent _returnvalue_4 (Variables|Default|GetW) "None" "SnapToTarget" "SnapToTarget" "KeepWorld" true)))))))

(fn ConstructionScript)