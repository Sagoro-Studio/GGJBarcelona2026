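; Interaction component that detects which "Interactable"-tagged actor the player is looking at and sends it hover and unhover messages.
; An overlap counter starts a looping sight-check timer while any interactable overlap is active and clears it otherwise.
; Each check sphere-traces on Visibility from the deprojected screen center, tracking the current target and CanInteract state.
; Debug trace drawing and a hover print are enabled.
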(event Custom|On%20Interactable%20Oberlap
  (params (Overlaps :type Boolean))
  (Utilities|FlowControl|Sequence
    (:then_0
      (Variables|Default|SetOverlapCount (+ (Variables|Default|GetOverlapCount) (select Overlaps 1 -1))))
    (:then_1
      (CallFunction|DrawTrace (> (Variables|Default|GetOverlapCount) 0)))))

(event Custom|Draw%20Trace
  (params (DrawTrace :type Boolean))
  (if DrawTrace
    (bind _returnvalue (Utilities|Time|SetTimerbyFunctionName 0 "Detect Sight" 0.1 true))
    (Variables|Default|SetTracTimer _returnvalue)
    (else
      (Utilities|Time|ClearandInvalidateTimerbyHandle (Variables|Default|GetTracTimer)))))

(event Custom|Detect%20Sight
  (bind (_outputpin _returnvalue) (CallFunction|CalculateTraceStartEnd))
  (bind (_outhit _returnvalue_2) (Collision|SphereTraceByChannel _outputpin _returnvalue 5.0 "TraceTypeQuery1" false 0 "ForDuration" true "(R=1.000000,G=0.000000,B=0.000000,A=1.000000)" "(R=0.000000,G=1.000000,B=0.000000,A=1.000000)" 0.1))
  (if _returnvalue_2
    (if (Actor|ActorHasTag (.HitActor (Collision|BreakHitResult _outhit)) "Interactable")
      (if (not (== (.HitActor (Collision|BreakHitResult _outhit)) (Variables|Default|GetInteractableObject)))
        (bind _interactableobject (Variables|Default|GetInteractableObject)
          (:then
            (Class|BPIInteractuable|OnUnhovered(Message) _interactableobject))
          (:else
            _))
        (Variables|Default|SetInteractableObject (.HitActor (Collision|BreakHitResult _outhit)))
        (Variables|Default|SetCanInteract true)
        (Class|BPIInteractuable|OnHovered(Message) (Variables|Default|GetInteractableObject))
        (Development|PrintString "Hello"))
      (else
        (if (Variables|Default|GetCanInteract) :!label _label
          (bind _interactableobject_2 (Variables|Default|GetInteractableObject)
            (:then
              (Class|BPIInteractuable|OnUnhovered(Message) _interactableobject_2))
            (:else
              _))
          (Variables|Default|SetInteractableObject 0)
          (Variables|Default|SetCanInteract false))))
    (else
      (goto _label))))

(fn CalculateTraceStartEnd
  (bind _returnvalue (Game|GetPlayerController 0))
  (bind (_sizex _sizey) (HUD|GetViewportSize _returnvalue))
  (bind _returnvalue_2 (/ _sizex 2))
  (bind _returnvalue_3 (/ _sizey 2))
  (bind _returnvalue_4 (Math|Conversions|ToFloat(Integer) _returnvalue_2))
  (bind _returnvalue_5 (Math|Conversions|ToFloat(Integer) _returnvalue_3))
  (bind (_worldlocation _worlddirection) (Class|PlayerController|DeprojectScreenPositiontoWorld _returnvalue _returnvalue_4 _returnvalue_5))
  (return _worldlocation (+ _worldlocation (* _worlddirection (Variables|Default|GetDistance)))))