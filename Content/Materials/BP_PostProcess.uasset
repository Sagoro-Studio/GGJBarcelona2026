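; BP_PostProcess is an experimental Blueprint that applies a post-process material at runtime when W is pressed.
; The press creates a dynamic material instance with no parent material specified, stores it in NewVar, and writes it as a weighted blendable into the PostProcess settings.
; A second W press handler writes to those settings without setting any members.
; The construction script is empty.
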(event Input|KeyboardEvents|W
  (params (Key :type Key%20Structure :default "None"))
  (:Pressed
    (Utilities|Struct|SetmembersinPostProcessSettings (Variables|/Script/Engine.PostProcessComponent|GetSettings (Variables|Default|GetPostProcess)) (Utilities|Struct|MakeWeightedBlendables 0))))

(event Input|KeyboardEvents|W
  (params (Key :type Key%20Structure :default "None"))
  ;[0.15 0.15 0.15 0.5] ?????????????????? Internet diu que se fa aixi?
  (:Pressed
    (bind _returnvalue (Rendering|Material|CreateDynamicMaterialInstance 0 "None" "None" :!class /Script/Engine.KismetMaterialLibrary))
    (bind _output_get (Variables|Default|SetNewVar _returnvalue))
    (Utilities|Struct|SetmembersinPostProcessSettings (Variables|/Script/Engine.PostProcessComponent|GetSettings (Variables|Default|GetPostProcess)) (Utilities|Struct|MakeWeightedBlendables (Utilities|Array|MakeArray (Utilities|Struct|MakeWeightedBlendable -1.0 _output_get))))))

(fn ConstructionScript)